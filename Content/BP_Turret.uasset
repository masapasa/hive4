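; Twin-barrel auto turret, set up as an AA gun, that tracks and shoots the nearest visible WorldDynamic actor within sensing range.
; Each Tick picks a target by sphere overlap and line of sight, rotates the top at constant speed with clamped pitch, and prints the target's name.
; Once cooled down and facing the target by dot product, it fires a DoN-looped burst of bullets, alternating barrels and playing curve-driven recoil timelines.
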(event `self.ReceiveBeginPlay`
  ;[1 1 1] Assign float curves on event play for animations
  (`TimelineComponent.SetFloatCurve` (`self.RecoilTimelineL`) "/Game/RecoilCurve.RecoilCurve" "Recoil")
  (`TimelineComponent.SetFloatCurve` (`self.RecoilTimelineR`) "/Game/RecoilCurve.RecoilCurve" "Recoil"))

(event `self.ReceiveTick`
  (params (DeltaSeconds :type "Float (single-precision)"))
  (`self.FindClosestTarget`)
  (`self.Target` ; is target valid?
    (:`then`
      (`self.UpdateTurretRotation` DeltaSeconds)
      (`self.UpdateFire`)
      (`KismetSystemLibrary.PrintString` (`KismetSystemLibrary.GetDisplayName` (`self.Target`))))
    (:`else`)))

(event `Fire`
  (set `self.TimeOfLastFire` (`KismetSystemLibrary.GetGameTimeInSeconds`))
  (`|ExecutionSequence`
    (:`then_0`
      (goto _label :!via `Reset`))
    (:`then_1`
      (`/Engine/EditorBlueprintResources/StandardMacros.Do N` 6 :!label _label
        (:`Exit`
          (`|SpawnActorFromClass` "/Game/Bullet.Bullet_C" (`SceneComponent.GetSocketTransform` (`self.StaticMeshBarrelL`) "Socket" "RTS_World") "Undefined" "OverrideRootScale" null 0.0 null)
          (`TimelineComponent.PlayFromStart` (`self.RecoilTimelineL`))
          (`KismetSystemLibrary.Delay` 0.2)
          (`|SpawnActorFromClass` "/Game/Bullet.Bullet_C" (`SceneComponent.GetSocketTransform` (`self.StaticMeshBarrelR`) "Socket" "RTS_World") "Undefined" "OverrideRootScale" null 0.0 null)
          (`TimelineComponent.PlayFromStart` (`self.RecoilTimelineR`))
          (`KismetSystemLibrary.Delay` 0.2)
          (goto _label))))))

(fn `FindClosestTarget`
  (locals (`Preferred Distance (local)` :type "Float (double-precision)") (`Current Distance (local)` :type "Float (double-precision)") (`Preferred Target (local)` :type "Actor Object Reference") (`Current Target (local)` :type "Actor Object Reference"))
  (set `local.Preferred Distance (local)` (+ (`self.Sensing Range`) 1.0))
  ;[1 1 1] Set the current target
  (bind _outactors (`KismetSystemLibrary.SphereOverlapActors` (`self.K2_GetActorLocation`) (`self.Sensing Range`) (`|MakeArray` "ObjectTypeQuery2" :!type "EObjectTypeQuery Enum") "/Script/Engine.Actor" (`|MakeArray` self :!type "Actor Object Reference")))
  (for _array_element _outactors
    (bind _output_get (set `local.Current Target (local)` _array_element))
    ;[1 1 1] Check which target is closest
    (bind _output_get_2 (set `local.Current Distance (local)` (`self.GetDistanceTo` _output_get self)))
    (if (or (< _output_get_2 (`local.Preferred Distance (local)`)) (not (`KismetSystemLibrary.IsValid` (`local.Preferred Target (local)`))))
      ;[1 1 1] Check if line of sight
      (bind _result (`/Game/MyFunctionLibrary.HasLineOfSight` (`SceneComponent.K2_GetComponentLocation` (`self.StaticMeshTop`)) (`self.K2_GetActorLocation` (`local.Current Target (local)`)) (`|MakeArray` self (`local.Current Target (local)`) :!type "Actor Object Reference"))) ; Determine Line of Sight
      (if _result
        ;[1 1 1] Set Preferred Target and Distance
        (set `local.Preferred Target (local)` (`local.Current Target (local)`))
        (set `local.Preferred Distance (local)` (`local.Current Distance (local)`)))))
  (set `self.Target` (`local.Preferred Target (local)`)))

(fn `UpdateFire`
  ;[1 1 1] Check if turret has cooled down enough before next fire
  (if (> (- (`KismetSystemLibrary.GetGameTimeInSeconds`) (`self.TimeOfLastFire`)) (`self.Rate of Fire`))
    ;[1 1 1] Check if turret is facing target via dot product before opening fire
    (if (> (`KismetMathLibrary.Dot_VectorVector` (`KismetMathLibrary.GetDirectionUnitVector` (`SceneComponent.K2_GetComponentLocation` (`self.StaticMeshTop`)) (`self.K2_GetActorLocation` (`self.Target`))) (`SceneComponent.GetForwardVector` (`self.StaticMeshTop`))) 0.95)
      (`self.Fire`))))

(fn `UpdateTurretRotation`
  (params (DeltaTime :type "Float (double-precision)"))
  (locals (NewRotation :type "Rotator Structure" :default (struct)))
  (bind _output_get (set `local.NewRotation` (`KismetMathLibrary.RInterpTo_Constant` (`SceneComponent.K2_GetComponentRotation` (`self.StaticMeshTop`)) (`KismetMathLibrary.FindLookAtRotation` (`SceneComponent.K2_GetComponentLocation` (`self.StaticMeshBarrelL`)) (`self.K2_GetActorLocation` (`self.Target`))) (`local.DeltaTime`) (`self.Rotation Speed`))))
  (`SceneComponent.K2_SetWorldRotation` (`self.StaticMeshTop`) (`KismetMathLibrary.MakeRotator` (.roll _output_get) (`KismetMathLibrary.ClampAngle` (.pitch _output_get) -45.0 75.0) (.yaw _output_get)) false false))

(fn `UserConstructionScript`)